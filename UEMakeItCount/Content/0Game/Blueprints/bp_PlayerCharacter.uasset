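; Networked top-down player character that carries and throws killer balls, with a billboarded name tag and customizable skin.
; UI events cycle head, armor and color indices, apply them and save to the game instance, from which they are sent to the server.
; Tick reapplies skins or a dead material based on IsAlive, which authority-only kill and revive events toggle along with collision.
; Balls spawn attached to the right hand, then detach and shoot via multicast.
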(event `self.ReceiveBeginPlay`
  ;[1 1 1] begin play
  (`|ExecutionSequence`
    (:`then_0`
      (`self.SetNameFromClient`))
    (:`then_1`
      ;[1 1 1] Init if Not Local Player
      (if (not (`Controller.IsLocalPlayerController` (`GameplayStatics.GetPlayerController` 0)))
        (`SceneComponent.SetHiddenInGame` (`self.CursorToWorld`) true true)
        (`ActorComponent.K2_DestroyComponent` (`self.TopDownCameraComponent`))
        (`ActorComponent.K2_DestroyComponent` (`self.CameraBoom`))))
    (:`then_2`
      (set `self.IsAlive` true))))

(event `self.ReceiveTick`
  (params (DeltaSeconds :type "Float (single-precision)"))
  (bind _textrender (`self.TextRender`))
  ;[1 1 1] Tick
  (`|ExecutionSequence`
    (:`then_0`
      (`TextRenderComponent.K2_SetText` _textrender (`KismetTextLibrary.Conv_StringToText` (`self.PlayerName`)))
      (`SceneComponent.K2_SetWorldRotation` _textrender (`KismetMathLibrary.Conv_VectorToRotator` (`KismetMathLibrary.GreaterGreater_VectorRotator` (`KismetMathLibrary.Normal` (- (`SceneComponent.K2_GetComponentLocation` (`self.TopDownCameraComponent`)) (`SceneComponent.K2_GetComponentLocation` _textrender))))) false false))
    (:`then_1`
      (if (not (`self.IsLocallyControlled`))
        (`SceneComponent.SetHiddenInGame` (`self.CursorToWorld`) true true)
        (if (not (`self.HasAuthority`))
          (`PrimitiveComponent.SetMaterial` (`self.Head_Accessory`) 0 (`|GetArrayItem` (`self.Colors`) (`self.index_Head_Color`))))))
    (:`then_2`
      (`|ExecutionSequence`
        (:`then_0`
          (if (`self.IsAlive`)
            (`self.SetSkinHead_Client`)
            (`self.SetSkinBody_Client`)
            (else
              (`PrimitiveComponent.SetMaterial` (`self.Mesh`) 0 (`self.MaterialDead`))
              (`PrimitiveComponent.SetMaterial` (`self.Head_Accessory`) 0 (`self.MaterialDead`))
              (`PrimitiveComponent.SetMaterial` (`self.Body_Accesory`) 0 (`self.MaterialDead`)))))))))

(event `SendLocalSkins_ToServer`
  ;[1 1 1] Send Local Skin Values To Server
  (if (`self.IsLocallyControlled`)
    (bind _asdb_game_instance (cast `DB_GameInstance` (`GameplayStatics.GetGameInstance`)))
    (`self.SetSkinValues_Onserver` (`KismetStringLibrary.Conv_StringToInt` (`DB_GameInstance.IndexSetup_HeadMesh` _asdb_game_instance)) (`KismetStringLibrary.Conv_StringToInt` (`DB_GameInstance.IndexSetup_HeadColor` _asdb_game_instance)) (`KismetStringLibrary.Conv_StringToInt` (`DB_GameInstance.IndexSetup_WholeBodyColor` _asdb_game_instance)) (`KismetStringLibrary.Conv_StringToInt` (`DB_GameInstance.IndexSetup_BodyMesh` _asdb_game_instance)) (`KismetStringLibrary.Conv_StringToInt` (`DB_GameInstance.IndexSetup_BodyColor` _asdb_game_instance)))))

(event `SelectIndex_HeadMesh`
  (params (next :type Boolean))
  (bind _index_head_mesh (`self.index_Head_Mesh`))
  (bind _index_head_mesh_2 (`self.index_Head_Mesh`))
  ;[1 1 1] Select Head Mesh From UI
  (if next
    (if (< _index_head_mesh (- (`KismetArrayLibrary.Array_Length` (`self.HeadMeshes`)) 1))
      (`/Engine/EditorBlueprintResources/StandardMacros.IncrementInt` _index_head_mesh
        (:`  `
          _))
      (else
        (set `self.index_Head_Mesh` 0)))
    (elif (> _index_head_mesh_2 0)
      (`/Engine/EditorBlueprintResources/StandardMacros.DecrementInt` _index_head_mesh_2
        (:`  `
          _))
      (else
        (set `self.index_Head_Mesh` (- (`KismetArrayLibrary.Array_Length` (`self.HeadMeshes`)) 1)))))
  (`self.SetSkinHead_Client`)
  (`self.Set_GameInstance_SkinData`))

(event `SetSkinValues_Onserver`
  (params (I_Head_Mesh :type Integer) (I_Head_Color :type Integer) (I_Body_Color :type Integer) (I_Armor_Mesh :type Integer) (I_Armor_Color :type Integer))
  ;[1 1 1] Set Skin Values in Server
  (set `self.index_Head_Mesh` I_Head_Mesh)
  (set `self.index_Head_Color` I_Head_Color)
  (set `self.index_BodySkin_Color` I_Body_Color)
  (set `self.index_BodyAccess_Mesh` I_Armor_Mesh)
  (set `self.index_BodyAccess_Color` I_Armor_Color)
  (`self.SetSkinHead_Client`)
  (`self.SetSkinBody_Client`))

(event `SetAnimPlayRate`
  (params (RAte :type "Float (double-precision)"))
  ;[1 1 1] Set Anim Play Rate
  (`SkeletalMeshComponent.SetPlayRate` (`self.Mesh`) RAte))

(event `SelectIndex_HeadColor`
  (params (next :type Boolean))
  (bind _index_head_color (`self.index_Head_Color`))
  (bind _index_head_color_2 (`self.index_Head_Color`))
  ;[1 1 1] Select Head Color From UI
  (if next
    (if (< _index_head_color_2 (- (`KismetArrayLibrary.Array_Length` (`self.Colors`)) 1))
      (`/Engine/EditorBlueprintResources/StandardMacros.IncrementInt` _index_head_color_2
        (:`  `
          _))
      (else
        (set `self.index_Head_Color` 0)))
    (elif (> _index_head_color 0)
      (`/Engine/EditorBlueprintResources/StandardMacros.DecrementInt` _index_head_color
        (:`  `
          _))
      (else
        (set `self.index_Head_Color` (- (`KismetArrayLibrary.Array_Length` (`self.Colors`)) 1)))))
  (`self.SetSkinHead_Client`)
  (`self.Set_GameInstance_SkinData`))

(event `SetSkinHead_Client`
  (bind _head_accessory (`self.Head_Accessory`))
  ;[1 1 1] Set Skin Head
  (`StaticMeshComponent.SetStaticMesh` _head_accessory (`|GetArrayItem` (`self.HeadMeshes`) (`self.index_Head_Mesh`)))
  (`PrimitiveComponent.SetMaterial` _head_accessory 0 (`|GetArrayItem` (`self.Colors`) (`self.index_Head_Color`))))

(event `SetName_InServer`
  (params (SetName :type String))
  ;[1 1 1] set name in server
  (set `self.PlayerName` SetName))

(event `SetNameFromClient`
  ;[1 1 1] set name from client
  (bind _asbp_game_instance (cast `/Game/0Game/Blueprints/bp_GameInstance` (`GameplayStatics.GetGameInstance`)))
  (`self.SetName_InServer` (`DB_GameInstance.PlayerName` _asbp_game_instance)))

(event `self.DoKill`
  ;[1 1 1] Do On Dead
  (if (`self.HasAuthority`)
    (set `self.IsAlive` false)
    (`self.SetActorEnableCollision` false)))

(event `SetSkinBody_Client`
  (bind _body_accesory (`self.Body_Accesory`))
  ;[1 1 1] Set Skin Body
  (`StaticMeshComponent.SetStaticMesh` _body_accesory (`|GetArrayItem` (`self.BodyMeshes`) (`self.index_BodyAccess_Mesh`)))
  (`PrimitiveComponent.SetMaterial` _body_accesory 0 (`|GetArrayItem` (`self.Colors`) (`self.index_BodyAccess_Color`)))
  (`PrimitiveComponent.SetMaterial` (`self.Mesh`) 0 (`|GetArrayItem` (`self.Colors`) (`self.index_BodySkin_Color`))))

(event `SelectIndex_ArmorMesh`
  (params (next :type Boolean))
  (bind _index_bodyaccess_mesh (`self.index_BodyAccess_Mesh`))
  (bind _index_bodyaccess_mesh_2 (`self.index_BodyAccess_Mesh`))
  ;[1 1 1] Select Armor Mesh From UI
  (if next
    (if (< _index_bodyaccess_mesh (- (`KismetArrayLibrary.Array_Length` (`self.BodyMeshes`)) 1))
      (`/Engine/EditorBlueprintResources/StandardMacros.IncrementInt` _index_bodyaccess_mesh
        (:`  `
          _))
      (else
        (set `self.index_BodyAccess_Mesh` 0)))
    (elif (> _index_bodyaccess_mesh_2 0)
      (`/Engine/EditorBlueprintResources/StandardMacros.DecrementInt` _index_bodyaccess_mesh_2
        (:`  `
          _))
      (else
        (set `self.index_BodyAccess_Mesh` (- (`KismetArrayLibrary.Array_Length` (`self.BodyMeshes`)) 1)))))
  (`self.SetSkinBody_Client`)
  (`self.Set_GameInstance_SkinData`))

(event `self.DoRevive`
  ;[1 1 1] Do Revive
  (if (`self.HasAuthority`)
    (set `self.IsAlive` true)
    (`self.SetActorEnableCollision` true)))

(event `self.GiveNewBall`
  ;[1 1 1] Give New Ball
  (if (`self.HasAuthority`)
    (`self.AddBall_Server`)))

(event `Set_GameInstance_SkinData`
  ;[1 1 1] Set Values in GameInstance
  (bind _asbp_game_instance (`self.GetDBGameInstance`))
  (set `DB_GameInstance.IndexSetup_HeadMesh` (`KismetStringLibrary.Conv_IntToString` (`self.index_Head_Mesh`)) _asbp_game_instance)
  (set `DB_GameInstance.IndexSetup_HeadColor` (`KismetStringLibrary.Conv_IntToString` (`self.index_Head_Color`)) _asbp_game_instance)
  (set `DB_GameInstance.IndexSetup_BodyMesh` (`KismetStringLibrary.Conv_IntToString` (`self.index_BodyAccess_Mesh`)) _asbp_game_instance)
  (set `DB_GameInstance.IndexSetup_BodyColor` (`KismetStringLibrary.Conv_IntToString` (`self.index_BodyAccess_Color`)) _asbp_game_instance)
  (set `DB_GameInstance.IndexSetup_WholeBodyColor` (`KismetStringLibrary.Conv_IntToString` (`self.index_BodySkin_Color`)) _asbp_game_instance))

(event `SelectIndex_ArmorColor`
  (params (next :type Boolean))
  (bind _index_bodyaccess_color (`self.index_BodyAccess_Color`))
  (bind _index_bodyaccess_color_2 (`self.index_BodyAccess_Color`))
  ;[1 1 1] Select Armor Color From UI
  (if next
    (if (< _index_bodyaccess_color_2 (- (`KismetArrayLibrary.Array_Length` (`self.Colors`)) 1))
      (`/Engine/EditorBlueprintResources/StandardMacros.IncrementInt` _index_bodyaccess_color_2
        (:`  `
          _))
      (else
        (set `self.index_BodyAccess_Color` 0)))
    (elif (> _index_bodyaccess_color 0)
      (`/Engine/EditorBlueprintResources/StandardMacros.DecrementInt` _index_bodyaccess_color
        (:`  `
          _))
      (else
        (set `self.index_BodyAccess_Color` (- (`KismetArrayLibrary.Array_Length` (`self.Colors`)) 1)))))
  (`self.SetSkinBody_Client`)
  (`self.Set_GameInstance_SkinData`))

(event `AddBall_Server`
  ;[1 1 1] add ball server
  (bind _returnvalue (`|SpawnActorFromClass` "/Game/0Game/Blueprints/bp_KillerBall.bp_KillerBall_C" (`KismetMathLibrary.MakeTransform` (0.0 0.0 0.0) (struct) (2.0 2.0 2.0)) "Undefined" "OverrideRootScale" self null))
  (`self.K2_AttachToComponent` _returnvalue (`self.Mesh`) "RightHand" "KeepRelative" "KeepRelative" "KeepRelative" true)
  (bind _output_get (set `self.CurrentBallInHand` _returnvalue))
  (`/Game/0Game/Blueprints/bp_KillerBall.Init` _output_get self))

(event `SelectIndex_BodySkinColor`
  (params (next :type Boolean))
  (bind _index_bodyskin_color (`self.index_BodySkin_Color`))
  (bind _index_bodyskin_color_2 (`self.index_BodySkin_Color`))
  ;[1 1 1] Select Skin Color From UI
  (if next
    (if (< _index_bodyskin_color_2 (- (`KismetArrayLibrary.Array_Length` (`self.Colors`)) 1))
      (`/Engine/EditorBlueprintResources/StandardMacros.IncrementInt` _index_bodyskin_color_2
        (:`  `
          _))
      (else
        (set `self.index_BodySkin_Color` 0)))
    (elif (> _index_bodyskin_color 0)
      (`/Engine/EditorBlueprintResources/StandardMacros.DecrementInt` _index_bodyskin_color
        (:`  `
          _))
      (else
        (set `self.index_BodySkin_Color` (- (`KismetArrayLibrary.Array_Length` (`self.Colors`)) 1)))))
  (`self.SetSkinBody_Client`)
  (`self.Set_GameInstance_SkinData`))

(event `self.OnShootDone`
  (params (TargetDirection :type "Vector Structure"))
  ;[1 1 1] on shoot done
  (`self.OnShootDone_MultiCast` TargetDirection))

(event `OnShootDone_MultiCast`
  (params (CursorPosition :type "Vector Structure"))
  (bind _currentballinhand (`self.CurrentBallInHand`))
  ;[1 1 1] on shoot done multicast
  (if (`KismetSystemLibrary.IsValid` (`self.CurrentBallInHand`))
    (`self.K2_DetachFromActor` _currentballinhand "KeepWorld" "KeepWorld" "KeepWorld")
    (`/Game/0Game/Blueprints/bp_KillerBall.Shoot` _currentballinhand CursorPosition)
    (set `self.CurrentBallInHand` null)))

(fn `OnRep_index_Head_Mesh`)

(fn `UserConstructionScript`
  (bind _head_accessory (`self.Head_Accessory`))
  (bind _body_accesory (`self.Body_Accesory`))
  (`|ExecutionSequence`
    (:`then_0`
      (`SceneComponent.K2_AttachToComponent` _head_accessory (`self.Mesh`) "Head" "KeepWorld" "KeepWorld" "KeepWorld" true)
      (`SceneComponent.K2_SetRelativeLocation` _head_accessory (0.0 0.0 0.0) false false)
      (`SceneComponent.K2_SetRelativeRotation` _head_accessory (struct :`Roll` -90.0) false false))
    (:`then_1`
      (`SceneComponent.K2_AttachToComponent` _body_accesory (`self.Mesh`) "Hips" "KeepWorld" "KeepWorld" "KeepWorld" true)
      (`SceneComponent.K2_SetRelativeLocation` _body_accesory (0.0 0.0 0.0) false false)
      (`SceneComponent.K2_SetRelativeRotation` _body_accesory (struct :`Roll` -90.0) false false))))