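; Game rules Blueprint that runs a server-started, round-based killer-ball match between players.
; StartMatch restarts music and resets players, then each round hands out balls and counts down with a self-calling Delay tick.
; On timeout, balls are destroyed and players revived for the next round.
; CheckWinner ends the match at the configured kill count, shows the winner, broadcasts through event dispatchers and restarts.
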(event `self.ReceiveBeginPlay`
  ;[1 1 1] Begin Play
  (`parent.ReceiveBeginPlay`)
  (if (`self.HasAuthority`)
    (`KismetSystemLibrary.Delay` 1.0)
    (`self.StartMatch`)))

(event `StartMatch`
  ;[1 1 1] Start Mach
  (`|ExecutionSequence`
    (:`then_0`
      (bind _outactors (`GameplayStatics.GetAllActorsWithTag` "MusicObject"))
      (bind _asbp_music (cast `/Game/0Game/Blueprints/bp_Music` (`|GetArrayItem` _outactors)))
      (`/Game/0Game/Blueprints/bp_Music.StartNewSong` _asbp_music))
    (:`then_1`
      (set `self.ThereIsWinner` false)
      (bind _outactors_2 (`GameplayStatics.GetAllActorsOfClass` "/Game/0Game/Blueprints/bp_PlayerCharacter.bp_PlayerCharacter_C"))
      (for _array_element _outactors_2
        (`UEMakeItCountCharacter.DoRevive` _array_element)
        (set `UEMakeItCountCharacter.QtyKills` 0 _array_element)
        (`/Game/0Game/Blueprints/bp_PlayerCharacter.SetCanMove_MultiCast` _array_element true)
        (`/Game/0Game/Blueprints/bp_PlayerCharacter.ShowGameplayCamera` _array_element)
        (`self.Dispatch_MatchStarted`)
        (`self.StartRound`)))))

(event `Dispatch_RoundAboutToStart`
  ;[1 1 1] Dispatch Round About To Start
  (`self.RoundAboutToStart`))

(event `StartRound`
  ;[1 1 1] Start Round
  (set `self.RoundCurrentTicks` (`self.RoundTotalTicks`))
  (`self.Dispatch_RoundAboutToStart`)
  (`KismetSystemLibrary.Delay` 1.5)
  (bind _outactors (`GameplayStatics.GetAllActorsOfClass` "/Game/0Game/Blueprints/bp_PlayerCharacter.bp_PlayerCharacter_C"))
  (for _array_element _outactors
    (`UEMakeItCountCharacter.GiveNewBall` _array_element))
  (`self.DoRoundTimerTick`))

(event `Dispatch_SomeoneWon`
  (params (PlayerName :type String) (QtyWins :type Integer))
  ;[1 1 1] Dispatch Someone Won
  (`self.SomeoneWon` PlayerName QtyWins))

(event `Dispatch_MatchStarted`
  ;[1 1 1] Dispatch Match Started
  (`self.MatchStarted`))

(event `DoRoundTimerTick`
  ;[1 1 1] Do Round Timer Tick
  (`KismetSystemLibrary.Delay` 1.0)
  (bind _result (`/Engine/EditorBlueprintResources/StandardMacros.DecrementInt` (`self.RoundCurrentTicks`))
    (:`  `
      (if (and (<= _result 0) (not (`self.ThereIsWinner`)))
        (`self.EndRound`)
        (else
          (`self.DoRoundTimerTick`))))))

(event `DestroyAllBalls`
  ;[1 1 1] Destroy All Balls
  (bind _outactors (`GameplayStatics.GetAllActorsOfClass` "/Game/0Game/Blueprints/bp_KillerBall.bp_KillerBall_C"))
  (bind (_arrayindex _arrayelement) (`/Engine/EditorBlueprintResources/StandardMacros.ReverseForEachLoop` _outactors)
    (:`LoopBody`
      (`self.K2_DestroyActor` _arrayelement))))

(event `EndRound`
  ;[1 1 1] End round
  (if (not (`self.ThereIsWinner`))
    (`|ExecutionSequence`
      (:`then_0`
        (`self.DestroyAllBalls`))
      (:`then_1`
        (bind _outactors (`GameplayStatics.GetAllActorsOfClass` "/Game/0Game/Blueprints/bp_PlayerCharacter.bp_PlayerCharacter_C"))
        (for _array_element _outactors
          (`UEMakeItCountCharacter.DoRevive` _array_element))
        (`KismetSystemLibrary.Delay` 2.0)
        (`self.StartRound`)))))

(event `CheckWinner`
  (bind _lastwinner (`self.LastWinner`))
  ;[1 1 1] CheckWinner
  (if (`self.HasAuthority`)
    (bind _outactors (`GameplayStatics.GetAllActorsOfClass` "/Game/0Game/Blueprints/bp_PlayerCharacter.bp_PlayerCharacter_C"))
    (for _array_element _outactors
      (if (>= (`UEMakeItCountCharacter.QtyKills` _array_element) (`DB_GameConfig.KillsToWin` (`self.GameConfig`)))
        ;[1 1 1] Show Winner and Dispatch End Match
        (`|ExecutionSequence`
          (:`then_0`
            (set `self.ThereIsWinner` true))
          (:`then_1`
            (bind _output_get (set `self.LastWinner` _array_element))
            (`/Engine/EditorBlueprintResources/StandardMacros.IncrementInt` (`UEMakeItCountCharacter.QtyMatchWins` _output_get)
              (:`  `
                (`/Game/0Game/Blueprints/bp_PlayerCharacter.ShowWinnerCamera` _output_get))))
          (:`then_2`
            (bind _outactors_2 (`GameplayStatics.GetAllActorsOfClass` "/Game/0Game/Blueprints/bp_PlayerCharacter.bp_PlayerCharacter_C"))
            (for _array_element_2 _outactors_2
              (`|ExecutionSequence`
                (:`then_0`
                  (if (not (== _array_element_2 (`self.LastWinner`)))
                    (`UEMakeItCountCharacter.DoKill` _array_element_2)))
                (:`then_1`
                  (`/Game/0Game/Blueprints/bp_PlayerCharacter.SetCanMove_MultiCast` _array_element_2 false)))))
          (:`then_3`
            (`self.DestroyAllBalls`))
          (:`then_5`
            (`self.Dispatch_SomeoneWon` (`UEMakeItCountCharacter.PlayerName` _lastwinner) (`UEMakeItCountCharacter.QtyMatchWins` _lastwinner))
            (`KismetSystemLibrary.Delay` 4.0)
            (`self.StartMatch`)))))))

(fn `UserConstructionScript`)