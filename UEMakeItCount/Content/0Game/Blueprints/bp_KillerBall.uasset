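; Killer ball projectile that a player shoots to kill other players, registering kills for its owner and asking GameRules to check for a winner.
; Once shot, Tick moves it horizontally toward the target point, and a trail is applied after one second, when self-hits become possible and cost a kill.
; Authority-gated overlaps destroy it on player kills, or line-trace non-player hits to reflect its direction until a rebound limit destroys it.
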(event `self.DoOnOverlapSomething`
  (params (OtherActor :type "Actor Object Reference") (SweepResult :type "HitResult Structure (by ref)"))
  (bind _movementdirection (`self.MovementDirection`))
  (bind _ownerplayerc (`self.OwnerPlayerC`))
  ;[1 1 1] Do On Overlap
  (if (`self.isMoving`)
    (if (`self.HasAuthority` (`GameplayStatics.GetPlayerController` 0))
      (bind _asbp_player_character (cast `/Game/0Game/Blueprints/bp_PlayerCharacter` OtherActor)
        (:`then`
          ;[1 1 1] Hit Against Players
          (if (!= _asbp_player_character (`self.OwnerPlayerC`))
            (`UEMakeItCountCharacter.RegisterKill` _ownerplayerc 1)
            (`UEMakeItCountCharacter.DoKill` _asbp_player_character :!label _label)
            (bind _outactors (`GameplayStatics.GetAllActorsWithTag` "GameRules"))
            (bind _asbp_game_rules (cast `/Game/0Game/Blueprints/bp_GameRules` (`|GetArrayItem` _outactors)))
            (`/Game/0Game/Blueprints/bp_GameRules.CheckWinner` _asbp_game_rules)
            (`self.K2_DestroyActor`)
            (elif (`self.CanImpactSelf`)
              (`UEMakeItCountCharacter.RegisterKill` _ownerplayerc -1)
              (goto _label))))
        (:`CastFailed`
          ;[1 1 1] Hit Against Walls
          (bind (_outhit _returnvalue) (`KismetSystemLibrary.LineTraceSingleForObjects` (`self.K2_GetActorLocation`) (+ (`self.K2_GetActorLocation`) (* (`KismetMathLibrary.Normal` (`self.MovementDirection`)) 2000.0)) (`|MakeArray` "ObjectTypeQuery1" "ObjectTypeQuery2" :!type "EObjectTypeQuery Enum") false (`|MakeArray` self :!type "Actor Object Reference")))
          (if _returnvalue
            (bind (_bblockinghit _binitialoverlap _time _distance _location _impactpoint _normal _impactnormal) (`GameplayStatics.BreakHitResult` _outhit))
            (set `self.MovementDirection` (- _movementdirection (* _impactnormal (* (`KismetMathLibrary.Dot_VectorVector` _movementdirection _impactnormal) 2.0))))
            (`/Engine/EditorBlueprintResources/StandardMacros.IncrementInt` (`self.Rebounds`)
              (:`  `
                (if (>= (`self.Rebounds`) (`self.MaxRebounds`))
                  (`self.K2_DestroyActor`))))))))))

(event `self.ReceiveBeginPlay`
  ;[1 1 1] Begin Play
  (`parent.ReceiveBeginPlay`)
  (set `self.isMoving` false))

(event `SetActorLocationEveryWhere`
  (params (Location :type "Vector Structure"))
  (`self.K2_SetActorLocation` self Location false false))

(event `self.ReceiveTick`
  (params (DeltaSeconds :type "Float (single-precision)"))
  ;[1 1 1] TICK
  (if (`self.isMoving`)
    (`self.SetActorLocationEveryWhere` self (+ (`self.K2_GetActorLocation` self) (* (`self.MovementDirection`) (* (`self.ShootSpeed`) DeltaSeconds))))))

(event `Init`
  (params (OwnerPlayerCharacter :type "/Game/0Game/Blueprints/bp_PlayerCharacter Object Reference"))
  ;[1 1 1] INIT
  (set `self.OwnerPlayerC` OwnerPlayerCharacter))

(event `Shoot`
  (params (Direction :type "Vector Structure"))
  (bind _returnvalue (`self.K2_GetActorLocation`))
  ;[1 1 1] Shoot
  (if (not (`self.isMoving`))
    (set `self.MovementDirection` (`KismetMathLibrary.Normal` (- (`KismetMathLibrary.MakeVector` (.x Direction) (.y Direction) (.z _returnvalue)) _returnvalue)))
    (set `self.isMoving` true)
    (`KismetSystemLibrary.Delay` 1.0)
    (set `self.CanImpactSelf` true)
    (`self.CreateTrail`)))

(event `CreateTrail`
  (`ParticleSystemComponent.SetTemplate` (`self.Trail`) "/Game/thirdPersonBP/Vfx/Trail.Trail"))

(fn `UserConstructionScript`)